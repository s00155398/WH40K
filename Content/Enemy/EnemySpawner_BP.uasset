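; EnemySpawner_BP is a spawner actor that keeps the level populated with Enemy_Bp actors up to MaxEnemiesAtATime.
; Tick counts all Enemy_Bp actors in the world and, while below the cap, runs a one-second Delay that throttles spawning.
; Each enemy spawns at a random point inside the Box component's bounds, with yaw from an unscaled RandomFloat (0 to 1 degree).
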(event EventBeginPlay)

(event Collision|EventActorBeginOverlap
  (params (OtherActor :type Actor%20Object%20Reference)))

(event EventTick
  (params (DeltaSeconds :type Float%20%28single-precision%29))
  (bind _box (Variables|Default|GetBox))
  (bind (_origin _boxextent) (Collision|GetComponentBounds _box))
  (bind _outactors (Actor|GetAllActorsOfClass "/Game/Enemy/Enemy_Bp.Enemy_Bp_C"))
  (if (< (Utilities|Array|Length _outactors) (Variables|Default|GetMaxEnemiesAtATime))
    (Utilities|FlowControl|Delay 1.0)
    (Game|SpawnActorfromClass "/Game/Enemy/Enemy_Bp.Enemy_Bp_C" (Math|Transform|MakeTransform (Math|Random|RandomPointinBoundingBox _origin _boxextent) (Math|Rotator|MakeRotator 0.0 0.0 (Math|Random|RandomFloat))) "Undefined" 0 0)))

(fn ConstructionScript)