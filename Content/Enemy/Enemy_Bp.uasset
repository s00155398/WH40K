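; Enemy character Blueprint for an AI-controlled zombie with a randomized look and a disintegrating death.
; BeginPlay randomly picks the skeletal mesh and one of two Anim Blueprints; only two of three mesh rolls are wired, so the third changes nothing.
; Die disables capsule collision and AI perception, stops and detaches the controller, then ragdolls the mesh.
; A timeline drives the dynamic material's dissolve amount, accompanied by an attached sound.
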(event Custom|Die
  (bind _returnvalue (Pawn|GetController))
  (Collision|SetCollisionEnabled (Variables|Collision|GetCapsuleComponent) "NoCollision")
  (bind _asenemy_ai_controller_bp (Utilities|Casting|CastToEnemy_Ai_Controller_BP _returnvalue))
  (Class|AIPerceptionComponent|SetSenseEnabled (Variables|/Game/ork/aI/Enemy_Ai_Controller_BP.Enemy_Ai_Controller_BP_C|GetAIPerception _asenemy_ai_controller_bp) "/Script/AIModule.AISense" false)
  (AI|Navigation|StopMovement _returnvalue)
  (Class|Pawn|DetachfromControllerPendingDestroy)
  (Physics|SetSimulatePhysics (Variables|Character|GetMesh) true)
  (bind _returnvalue_2 (Rendering|Material|CreateDynamicMaterialInstance (Variables|Character|GetMesh) 0 0 "None" :!class /Script/Engine.PrimitiveComponent))
  (Audio|SpawnSoundAttached "/Game/Audio/Disintegrate_Cue.Disintegrate_Cue" (Variables|Character|GetMesh) "None" "0, 0, 0" "0, 0, 0" "KeepRelativeOffset" false 1.0 1.0 0.0 0 0)
  (bind _newtrack_0 (Timeline|Disintegrate%20TimeLine Play)
    (:Update
      (Rendering|Material|SetScalarParameterValue _returnvalue_2 "Amount" _newtrack_0 :!class /Script/Engine.MaterialInstanceDynamic))))

(event EventTick
  (params (DeltaSeconds :type Float%20%28single-precision%29)))

(event Collision|EventActorBeginOverlap
  (params (OtherActor :type Actor%20Object%20Reference)))

(event EventBeginPlay
  (bind _mesh (Variables|Character|GetMesh))
  (Variables|Default|SetRanAnimNum (Math|Random|RandomIntegerinRange 0 1))
  (bind _output_get (Variables|Default|SetRanCharNum (Math|Random|RandomIntegerinRange 0 2)))
  (switch int _output_get
    (:0
      (Class|SkinnedMeshComponent|SetSkeletalMesh _mesh "/Game/Enemy/Type1/yaku_j_ignite.yaku_j_ignite" true))
    (:1
      (Class|SkinnedMeshComponent|SetSkeletalMesh _mesh "/Game/Enemy/Type2/warzombie_f_pedroso.warzombie_f_pedroso" true)))
  (switch int (Variables|Default|GetRanAnimNum)
    (:0
      (Class|SkeletalMeshComponent|SetAnimClass (Variables|Character|GetMesh) "/Game/Enemy/Animations/Enemy_Anim_BP.Enemy_Anim_BP_C"))
    (:1
      (Class|SkeletalMeshComponent|SetAnimClass (Variables|Character|GetMesh) "/Game/Enemy/Animations/Enemy_Anim_Alt_BP.Enemy_Anim_Alt_BP_C"))))

(fn ConstructionScript)