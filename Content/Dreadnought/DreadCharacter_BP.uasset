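; Player-controlled Dreadnought character with an independently aimed torso and gun arm and a spinning-barrel cannon.
; Look input turns the torso and pitches the gun arm; movement follows torso yaw, with a timeline easing the legs toward Arrow1's heading.
; Right mouse swaps the camera between spring arms and spins the barrel; left mouse also fires.
; Tick rotates the barrel and uses a Delay to pace projectile spawns, muzzle flashes and CannonBlast playback.
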(event Custom|RotateToRight)

(event Custom|RotateToLeft)

(event EventBeginPlay)

(event Collision|EventActorBeginOverlap
  (params (OtherActor :type Actor%20Object%20Reference)))

(event EventTick
  (params (DeltaSeconds :type Float%20%28single-precision%29))
  (Variables|Default|SetDeltaSeconds DeltaSeconds)
  (if (Variables|Default|GetIsSpinning)
    (Transformation|AddLocalRotation (Variables|Default|GetGun_Barrel) (Math|Rotator|MakeRotator 0.0 (* DeltaSeconds 2e+03) 0.0) false false)
    (if (Variables|Default|GetisFiring)
      (Utilities|FlowControl|Delay 0.1)
      (Audio|Components|Audio|Play (Variables|Default|GetCannonBlast) 0.0)
      (Game|SpawnActorfromClass "/Game/FireCaste/Projectile_BP.Projectile_BP_C" (Math|Transform|MakeTransform (Transformation|GetSocketLocation (Variables|Default|GetGun_Arm) "BolterBarrel") (Transformation|GetWorldRotation (Variables|Default|GetArrow1)) "0.100000,0.100000,0.100000") "AdjustIfPossibleButAlwaysSpawn" self 0)
      (Effects|SpawnEmitteratLocation "/Game/FXVarietyPack/Particles/P_ky_muzzleflash.P_ky_muzzleflash" (Transformation|GetSocketLocation (Variables|Default|GetGun_Arm) "BolterBarrel") "0, 0, 0" "0.050000,0.050000,0.050000"))))

(event Input|AxisEvents|InputAxisTurnRight
  (params (AxisValue :type Float%20%28single-precision%29))
  ;[1 1 1] Gun Arm Turn Axis
  (Transformation|AddRelativeRotation (Variables|Default|GetTorso) (Math|Rotator|MakeRotator 0.0 0.0 (* AxisValue (Utilities|Time|GetWorldDeltaSeconds) (Variables|Default|GetBaseTurnRate))) false false))

(event Input|AxisEvents|InputAxisTurnUp
  (params (AxisValue :type Float%20%28single-precision%29))
  ;[1 1 1] Gun Arm Turn Axis
  (Transformation|AddRelativeRotation (Variables|Default|GetGun_Arm) (Math|Rotator|MakeRotator (* AxisValue (Utilities|Time|GetWorldDeltaSeconds) (Variables|Default|GetBaseTurnRate)) 0.0 0.0) false false))

(event Input|AxisEvents|InputAxisMoveForward
  (params (AxisValue :type Float%20%28single-precision%29))
  (bind _mesh (Variables|Character|GetMesh))
  (Pawn|Input|AddMovementInput (Math|Vector|GetForwardVector (Math|Rotator|MakeRotator 0.0 0.0 (.Yaw (Math|Rotator|BreakRotator (Variables|/Script/Engine.SceneComponent|GetRelativeRotation (Variables|Default|GetTorso)))))) AxisValue false)
  (if (not (Math|Float|InRange(Float) AxisValue -0.9 0.9))
    (Timeline|RotateLegs Play
      (:Update
        (Transformation|SetWorldRotation _mesh (Math|Interpolation|RInterpTo (Transformation|GetWorldRotation _mesh) (Math|Rotator|MakeRotator 0.0 0.0 (+ (.Yaw (Math|Rotator|BreakRotator (Transformation|GetWorldRotation (Variables|Default|GetArrow1)))) 2.7e+02)) (Variables|Default|GetDeltaSeconds) (Variables|Default|GetLegTurnRate)) false false)))))

(event Input|AxisEvents|InputAxisMoveRight
  (params (AxisValue :type Float%20%28single-precision%29))
  (bind _mesh (Variables|Character|GetMesh))
  (Pawn|Input|AddMovementInput (Math|Vector|GetRightVector (Math|Rotator|MakeRotator 0.0 0.0 (.Yaw (Math|Rotator|BreakRotator (Variables|/Script/Engine.SceneComponent|GetRelativeRotation (Variables|Default|GetTorso)))))) AxisValue false)
  (if (not (Math|Float|InRange(Float) AxisValue -0.9 0.9))
    (Timeline|RotateLegs Play
      (:Update
        (Transformation|SetWorldRotation _mesh (Math|Interpolation|RInterpTo (Transformation|GetWorldRotation _mesh) (Math|Rotator|MakeRotator 0.0 0.0 (+ (.Yaw (Math|Rotator|BreakRotator (Transformation|GetWorldRotation (Variables|Default|GetArrow1)))) 2.7e+02)) (Variables|Default|GetDeltaSeconds) (Variables|Default|GetLegTurnRate)) false false)))))

(event Input|MouseEvents|LeftMouseButton
  (params (Key :type Key%20Structure))
  (:Pressed
    (Variables|Default|SetIsSpinning true)
    (Variables|Default|SetisFiring true)
    (Audio|Components|Audio|Play (Variables|Default|GetSpin) 0.0))
  (:Released
    (if (Game|Player|IsInputKeyDown (Game|GetPlayerController 0) "RightMouseButton")
      (Variables|Default|SetisFiring false)
      (else
        (Variables|Default|SetisFiring false)
        (Variables|Default|SetIsSpinning false)
        (Audio|Components|Audio|Stop (Variables|Default|GetSpin))))))

(event Input|MouseEvents|RightMouseButton
  (params (Key :type Key%20Structure))
  ;[1 1 1] Smooth Zoom
  (:Pressed
    (Transformation|AttachComponentToComponent (Variables|Default|GetCamera) (Variables|Default|GetSpringArm1) "None" "KeepRelative" "KeepRelative" "KeepRelative" true)
    (Variables|Default|SetIsSpinning true)
    (Audio|Components|Audio|Play (Variables|Default|GetSpin) 0.0))
  (:Released
    (Transformation|AttachComponentToComponent (Variables|Default|GetCamera) (Variables|Default|GetSpringArm) "None" "KeepRelative" "KeepRelative" "KeepRelative" true)
    (if (not (Game|Player|IsInputKeyDown (Game|GetPlayerController 0) "LeftMouseButton"))
      (Variables|Default|SetisFiring false)
      (Variables|Default|SetIsSpinning false)
      (Audio|Components|Audio|Stop (Variables|Default|GetSpin)))))

(fn ConstructionScript)