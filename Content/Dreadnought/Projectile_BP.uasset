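; Projectile actor that explodes on overlap and kills enemies it hits.
; Its capsule overlap spawns a half-scale explosion emitter and checks the sweep result's hit actor for the "Enemy" tag.
; A tagged Enemy_Bp gets Die and mesh physics simulation for a ragdoll.
; Successful hits and untagged overlaps both fire a radial force impulse and destroy the projectile, which otherwise expires on a timer from BeginPlay.
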(event OnComponentBeginOverlap(Capsule)
  (params (OverlappedComponent :type Primitive%20Component%20Object%20Reference) (OtherActor :type Actor%20Object%20Reference) (OtherComp :type Primitive%20Component%20Object%20Reference) (OtherBodyIndex :type Integer) (bFromSweep :type Boolean) (SweepResult :type Hit%20Result%20Structure%20%28by%20ref%29))
  (bind _hitactor (Collision|BreakHitResult SweepResult))
  (Effects|SpawnEmitteratLocation "/Game/FXVarietyPack/Particles/P_ky_explosion.P_ky_explosion" (Transformation|GetActorLocation) "0, 0, 0" "0.500000,0.500000,0.500000")
  (if (Actor|ActorHasTag _hitactor "Enemy")
    (bind _asenemy_bp (Utilities|Casting|CastToEnemy_Bp _hitactor))
    (bind _output_get (Variables|Default|SetHitEnemyRef _asenemy_bp))
    (Default|Die _output_get)
    (Physics|SetSimulatePhysics (Variables|/Script/Engine.Character|GetMesh _output_get) true))
  (Class|RadialForceComponent|FireImpulse (Variables|Default|GetRadialForce))
  (Actor|DestroyActor))

(event EventBeginPlay
  (Utilities|FlowControl|Delay 1e+01)
  (Actor|DestroyActor))

(event Collision|EventActorBeginOverlap
  (params (OtherActor :type Actor%20Object%20Reference)))

(event EventTick
  (params (DeltaSeconds :type Float%20%28single-precision%29)))

(fn ConstructionScript)