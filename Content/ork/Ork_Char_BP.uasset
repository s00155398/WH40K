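; Ork character Blueprint that handles a two-step melee combo and picks random roaming destinations.
; Attack alternates between a fast and a regular primary attack montage, tracked by AttackCount.
; Attacks requested mid-swing are buffered in SaveAttack, which ComboAttackSave consumes to chain the next montage, while ResetCombo clears the combo state.
; GetNextLocation returns a random reachable navigation point within a radius of the Ork's location.
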(event Custom|Attack
  (if (Variables|Default|GetIsAttacking)
    (Variables|Default|SetSaveAttack true)
    (else
      (Variables|Default|SetIsAttacking true)
      (switch int (Variables|Default|GetAttackCount)
        (:0
          (Variables|Default|SetAttackCount 1)
          (Animation|PlayAnimMontage "/Game/ork/Animations/PrimaryAttack_RA_Fast_Montage.PrimaryAttack_RA_Fast_Montage" 1.0 "None"))
        (:1
          (Variables|Default|SetAttackCount 0)
          (Animation|PlayAnimMontage "/Game/ork/Animations/PrimaryAttack_RA_Montage.PrimaryAttack_RA_Montage" 1.0 "None"))))))

(event Custom|ResetCombo
  (Variables|Default|SetAttackCount 0)
  (Variables|Default|SetSaveAttack false)
  (Variables|Default|SetIsAttacking false))

(event Custom|ComboAttackSave
  (if (Variables|Default|GetSaveAttack)
    (Variables|Default|SetSaveAttack false)
    (switch int (Variables|Default|GetAttackCount)
      (:0
        (Variables|Default|SetAttackCount 1)
        (Animation|PlayAnimMontage "/Game/ork/Animations/PrimaryAttack_RA_Fast_Montage.PrimaryAttack_RA_Fast_Montage" 1.0 "None"))
      (:1
        (Variables|Default|SetAttackCount 0)
        (Animation|PlayAnimMontage "/Game/ork/Animations/PrimaryAttack_RA_Montage.PrimaryAttack_RA_Montage" 1.0 "None")))))

(event EventBeginPlay)

(event Collision|EventActorBeginOverlap
  (params (OtherActor :type Actor%20Object%20Reference)))

(event EventTick
  (params (DeltaSeconds :type Float%20%28single-precision%29)))

(fn ConstructionScript)

(fn GetNextLocation
  (return (.RandomLocation (AI|Navigation|GetRandomReachablePointinRadius (Transformation|GetActorLocation) 2e+03 0 0))))