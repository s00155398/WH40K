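; ShootaProjectile_BP is a Shoota projectile actor that damages the player's Fire Warrior on contact.
; Its capsule overlap checks the hit actor for the Player tag, then spawns a character-hit effect and calls HitByChoppa on the Fire Warrior.
; Any other overlap spawns a world-hit effect, and both paths destroy the projectile.
; A delay on BeginPlay also destroys it if it hits nothing within its lifetime.
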(event OnComponentBeginOverlap(Capsule)
  (params (OverlappedComponent :type Primitive%20Component%20Object%20Reference) (OtherActor :type Actor%20Object%20Reference) (OtherComp :type Primitive%20Component%20Object%20Reference) (OtherBodyIndex :type Integer) (bFromSweep :type Boolean) (SweepResult :type Hit%20Result%20Structure%20%28by%20ref%29))
  (if (Actor|ActorHasTag (.HitActor (Collision|BreakHitResult SweepResult)) "Player")
    (bind _asmy_fire_warrior_character (Utilities|Casting|CastToMyFireWarrior_Character OtherActor))
    (Effects|SpawnEmitteratLocation "/Game/ork/ShootaBoy/P_ShootaHitCharacter.P_ShootaHitCharacter" (Transformation|GetActorLocation) "0.000000,90.000000, 0" "0.100000,0.100000,0.100000")
    (Class|FireWarriorCharacter|HitbyChoppa _asmy_fire_warrior_character)
    (else
      (Effects|SpawnEmitteratLocation "/Game/ork/ShootaBoy/P_Shoota_HitWorld.P_Shoota_HitWorld" (Transformation|GetActorLocation))))
  (Actor|DestroyActor))

(event EventBeginPlay
  (Utilities|FlowControl|Delay 1e+01)
  (Actor|DestroyActor))

(event Collision|EventActorBeginOverlap
  (params (OtherActor :type Actor%20Object%20Reference)))

(event EventTick
  (params (DeltaSeconds :type Float%20%28single-precision%29)))

(fn ConstructionScript)