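; AI controller for the Ork ShootaBoy character that drives its behavior and aiming.
; On BeginPlay it runs the ShootaBoy behavior tree and caches the controlled pawn.
; AI perception updates for Player-tagged actors set the TargetToFollow blackboard key and turn on the pawn's IsAiming, while other actors turn aiming off.
; It ignores whether the stimulus was gained or lost, and never clears the target.
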(event EventBeginPlay
  (AI|RunBehaviorTree "/Game/ork/ShootaBoy/Ai/Ork_ShootaBoy_BT.Ork_ShootaBoy_BT")
  (bind _asork_character_shoota_boy_bp (Utilities|Casting|CastToOrk_Character_ShootaBoy_BP (Pawn|GetControlledPawn)))
  (Variables|Default|SetControlledPawnRef _asork_character_shoota_boy_bp))

(event EventTick
  (params (DeltaSeconds :type Float%20%28single-precision%29)))

(event OnTargetPerceptionUpdated(AIPerception)
  (params (Actor :type Actor%20Object%20Reference) (Stimulus :type AI%20Stimulus%20Structure))
  (if (Actor|ActorHasTag Actor "Player")
    (AI|Components|Blackboard|SetValueasObject (Variables|Default|GetBlackboard) (Variables|Default|GetTargetToFollow) Actor)
    (Variables|/Script/WH40K.Ork_Character_ShootaBoy|SetIsAiming (Variables|Default|GetControlledPawnRef) true)
    (else
      (Variables|/Script/WH40K.Ork_Character_ShootaBoy|SetIsAiming (Variables|Default|GetControlledPawnRef) false))))

(fn ConstructionScript)