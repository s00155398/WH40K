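; Ork Shoota Boy character Blueprint, an armed Ork that supplies aim, movement and weapon socket data.
; Aim rotation faces the Opponent, falling back to its own rotation, and the next location is a random reachable point around it.
; Socket transforms come from the Shoota component, and recoil hits route to HitByProjectile.
; A timeline drives disintegration through each mesh material's Amount parameter, calling CreateDynamicMaterialInstance on every update.
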(event EventBeginPlay)

(event Collision|EventActorBeginOverlap
  (params (OtherActor :type Actor%20Object%20Reference)))

(event EventTick
  (params (DeltaSeconds :type Float%20%28single-precision%29)))

(event EventInitiateDisintegration
  (bind _disintegration (Timeline|Disintegration%20Timeline Play)
    (:Update
      (for (_array_element _array_index) (Rendering|Material|GetMaterials (Variables|Character|GetMesh))
        (bind _returnvalue (Rendering|Material|CreateDynamicMaterialInstance (Variables|Character|GetMesh) _array_index _array_element "None" :!class /Script/Engine.PrimitiveComponent))
        (Rendering|Material|SetScalarParameterValue _returnvalue "Amount" _disintegration :!class /Script/Engine.MaterialInstanceDynamic)))))

(event EventHitbyRecoil
  (Class|OrkCharacterShootaBoy|HitbyProjectile))

(fn ConstructionScript)

(fn GetAimingRotation
  (bind _opponent (Variables|Default|GetOpponent))
  (Utilities|IsValid _opponent
    (:Is%20Valid
      (return (Math|Rotator|FindLookatRotation (Transformation|GetActorLocation) (Transformation|GetActorLocation _opponent))))
    (:Is%20Not%20Valid
      (return (Transformation|GetActorRotation)))))

(fn GetNextLocation
  (return (.RandomLocation (AI|Navigation|GetRandomReachablePointinRadius (Transformation|GetActorLocation) 2e+03 0 0))))

(fn GetWeaponSocket
  (params (SocketName :type Name :default "None"))
  (return (Transformation|GetSocketTransform (Variables|Default|GetShoota) SocketName "RTS_World")))