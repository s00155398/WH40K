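; AI Controller for the OrkBoy enemy that starts its behavior tree and gives it the player as a target.
; Perception updates write any valid actor tagged Player into the TargetToFollow blackboard key, without checking whether it was sensed or lost.
; A ranged-attack alert event sets the same key directly to the first player character.
; The node that would clear the target is unconnected, so this controller never clears it.
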(event EventBeginPlay
  (AI|RunBehaviorTree "/Game/ork/OrkBoy/Ai/OrkBoy_BT.OrkBoy_BT"))

(event EventTick
  (params (DeltaSeconds :type Float%20%28single-precision%29)))

(event OnTargetPerceptionUpdated(AIPerception)
  (params (Actor :type Actor%20Object%20Reference) (Stimulus :type AI%20Stimulus%20Structure))
  (Utilities|IsValid Actor
    (:Is%20Valid
      (if (Actor|ActorHasTag Actor "Player")
        (AI|Components|Blackboard|SetValueasObject (Variables|Default|GetBlackboard) (Variables|Default|GetTargetToFollow) Actor)))))

(event Custom|AlertedByRangedAttack
  (AI|Components|Blackboard|SetValueasObject (Variables|Default|GetBlackboard) (Variables|Default|GetTargetToFollow) (Game|GetPlayerCharacter 0)))

(fn ConstructionScript)