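; Ork boy character Blueprint that responds to recoil hits, attacks and disintegrates.
; Hit and attack events forward to HitByProjectile and AttackInitiated.
; Disintegration plays a timeline that, on every update, creates dynamic instances of all mesh materials and drives their Amount parameter.
; GetNextLocation returns a random reachable point within a radius of the ork, apparently for roaming.
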(event EventBeginPlay)

(event Collision|EventActorBeginOverlap
  (params (OtherActor :type Actor%20Object%20Reference)))

(event EventTick
  (params (DeltaSeconds :type Float%20%28single-precision%29)))

(event EventHitbyRecoil
  (Class|OrkCharacterOrkBoy|HitbyProjectile))

(event EventAttack
  (Class|OrkCharacterOrkBoy|AttackInitiated))

(event EventInitiateDisintegration
  (bind _disintegration (Timeline|Disintegration%20%20Timeline Play)
    (:Update
      (for (_array_element _array_index) (Rendering|Material|GetMaterials (Variables|Character|GetMesh))
        (bind _returnvalue (Rendering|Material|CreateDynamicMaterialInstance (Variables|Character|GetMesh) _array_index _array_element "None" :!class /Script/Engine.PrimitiveComponent))
        (Rendering|Material|SetScalarParameterValue _returnvalue "Amount" _disintegration :!class /Script/Engine.MaterialInstanceDynamic)))))

(fn ConstructionScript)

(fn GetNextLocation
  (return (.RandomLocation (AI|Navigation|GetRandomReachablePointinRadius (Transformation|GetActorLocation) 2e+03 0 0))))