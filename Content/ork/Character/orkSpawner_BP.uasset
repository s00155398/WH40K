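; Spawner actor that keeps the level populated with Ork AI, either OrkBoys or ShootaBoys.
; Tick counts all actors of both classes and, while the total is at or below MaxNum, waits on a short Delay, spawns one, then loops back to recheck.
; Each spawn randomly picks one of the two classes, starts it with its own behavior tree and places it at a random point inside the Box component.
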(event Custom|Spawn%20boys
  (bind _box (Variables|Default|GetBox))
  (bind _returnvalue (Transformation|GetWorldLocation _box))
  (bind _boxextent (Variables|/Script/Engine.BoxComponent|GetBoxExtent _box))
  (bind _returnvalue_2 (Math|Random|RandomPointinBoundingBox _returnvalue _boxextent))
  (bind _output_get (Variables|Default|Setspawnnum (Math|Random|RandomIntegerinRange 0 1)))
  (if (== _output_get 0)
    (AI|SpawnAIFromClass "/Game/ork/Character/Ork_Character_OrkBoy_BP.Ork_Character_OrkBoy_BP_C" "/Game/ork/OrkBoy/Ai/OrkBoy_BT.OrkBoy_BT" _returnvalue_2 "0, 0, 0" false 0)
    (else
      (AI|SpawnAIFromClass "/Game/ork/Character/Ork_Character_ShootaBoy_BP.Ork_Character_ShootaBoy_BP_C" "/Game/ork/ShootaBoy/Ai/Ork_ShootaBoy_BT.Ork_ShootaBoy_BT" _returnvalue_2 "0, 0, 0" false 0))))

(event Collision|EventActorBeginOverlap
  (params (OtherActor :type Actor%20Object%20Reference)))

(event EventTick
  (params (DeltaSeconds :type Float%20%28single-precision%29))
  (bind _outactors (Actor|GetAllActorsOfClass "/Game/ork/Character/Ork_Character_OrkBoy_BP.Ork_Character_OrkBoy_BP_C" :!label _label))
  (bind _outactors_2 (Actor|GetAllActorsOfClass "/Game/ork/Character/Ork_Character_ShootaBoy_BP.Ork_Character_ShootaBoy_BP_C"))
  (if (<= (+ (Utilities|Array|Length _outactors_2) (Utilities|Array|Length _outactors)) (Variables|Default|GetmaxNum))
    (Utilities|FlowControl|Delay 2.0)
    (CallFunction|SpawnBoys)
    (goto _label)))

(fn ConstructionScript)