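; Ork Shoota Boy character, an AI-controlled ranged enemy with helpers for aiming at its opponent, random roam points and weapon socket transforms.
; Tick plays FMOD audio while it fires, alive and unstunned.
; HitbyRecoil alerts its AI controller before applying projectile damage.
; Disintegration spawns an emitter, then a timeline drives an "Amount" parameter on mesh and instanced-mesh materials, creating dynamic instances each update, before destroying the actor.
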(event EventTick
  (params (DeltaSeconds :type Float%20%28single-precision%29))
  (if (Math|Boolean|ANDBoolean (Variables|Default|GetIsFiring) (not (<= (Variables|Default|GetHealth) 0.0)) (not (Variables|Default|GetIsStunned)))
    (bind _returnvalue (Class|FMODAudioComponent|IsPlaying (Variables|Default|GetFMODAudio)))
    (if (not _returnvalue)
      (Class|FMODAudioComponent|Play (Variables|Default|GetFMODAudio)))
    (else
      (Class|FMODAudioComponent|Stop (Variables|Default|GetFMODAudio)))))

(event EventInitiateDisintegration
  (Effects|SpawnEmitteratLocation "/Game/FXVarietyPack/Particles/P_ky_waterBallHit.P_ky_waterBallHit" (Transformation|GetActorLocation))
  (bind _disintegration (Timeline|Disintegration%20Timeline Play)
    (:Update
      (|Disintegrate _disintegration))
    (:Finished
      (Actor|DestroyActor))))

(event EventHitbyRecoil
  (params (Damage :type Float%20%28single-precision%29))
  (bind _asork_shoota_boy_ai_controller_bp (Utilities|Casting|CastToOrk_ShootaBoy_Ai_Controller_BP (AI|GetAIController self)))
  (Default|AlertedbyRangedAttack _asork_shoota_boy_ai_controller_bp)
  (Class|OrkCharacterShootaBoy|HitbyProjectile Damage))

(fn ConstructionScript)

(fn GetAimingRotation
  (bind _opponent (Variables|Default|GetOpponent))
  (Utilities|IsValid _opponent
    (:Is%20Valid
      (return (Math|Rotator|FindLookatRotation (Transformation|GetActorLocation) (Transformation|GetActorLocation _opponent))))
    (:Is%20Not%20Valid
      (return (Transformation|GetActorRotation)))))

(fn GetNextLocation
  (return (.RandomLocation (AI|Navigation|GetRandomReachablePointinRadius (Transformation|GetActorLocation) 2e+03 0 0))))

(fn GetWeaponSocket
  (params (SocketName :type Name :default "None"))
  (return (Transformation|GetSocketTransform (Variables|Default|GetShoota) SocketName "RTS_World")))