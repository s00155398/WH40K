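; Ork Boy enemy character Blueprint that forwards attacks, reacts to ranged hits and disintegrates before being destroyed.
; Recoil hits alert its AI controller and pass damage to HitByProjectile, while GetNextLocation supplies a random reachable point around it.
; Disintegration spawns a particle burst, then a timeline drives the "Amount" material parameter on the mesh and instanced static meshes, calling CreateDynamicMaterialInstance on every update.
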(event EventBeginPlay)

(event Collision|EventActorBeginOverlap
  (params (OtherActor :type Actor%20Object%20Reference)))

(event EventTick
  (params (DeltaSeconds :type Float%20%28single-precision%29)))

(event EventHitbyRecoil
  (params (Damage :type Float%20%28single-precision%29))
  (bind _asork_boy_ai_controller_bp (Utilities|Casting|CastToOrkBoy_Ai_Controller_BP (AI|GetAIController self)))
  (Default|AlertedbyRangedAttack _asork_boy_ai_controller_bp)
  (Class|OrkCharacterOrkBoy|HitbyProjectile Damage))

(event EventAttack
  (Class|OrkCharacterOrkBoy|AttackInitiated))

(event EventInitiateDisintegration
  (Effects|SpawnEmitteratLocation "/Game/FXVarietyPack/Particles/P_ky_waterBallHit.P_ky_waterBallHit" (Transformation|GetActorLocation))
  (bind _disintegration (Timeline|Disintegration%20%20Timeline Play)
    (:Update
      (|Disintegrate _disintegration _disintegration))
    (:Finished
      (Actor|DestroyActor))))

(fn ConstructionScript)

(fn GetNextLocation
  (return (.RandomLocation (AI|Navigation|GetRandomReachablePointinRadius (Transformation|GetActorLocation) 2e+03 0 0))))