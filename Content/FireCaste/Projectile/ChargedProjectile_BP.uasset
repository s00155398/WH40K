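; Charged carbine projectile whose damage and size scale with CarbineChargeValue, self-destroying after ten seconds.
; Overlapping an Enemy-tagged actor spawns a charge-scaled explosion, then, if it casts to Ork_Character, stuns it at high charge, sends damage through HitByRecoilMessage and destroys the projectile.
; Other overlaps only spawn an unscaled explosion with no location wired, leaving the projectile alive.
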(event OnComponentBeginOverlap(Capsule)
  (params (OverlappedComponent :type Primitive%20Component%20Object%20Reference) (OtherActor :type Actor%20Object%20Reference) (OtherComp :type Primitive%20Component%20Object%20Reference) (OtherBodyIndex :type Integer) (bFromSweep :type Boolean) (SweepResult :type Hit%20Result%20Structure%20%28by%20ref%29))
  (if (Actor|ActorHasTag (.HitActor (Collision|BreakHitResult SweepResult)) "Enemy")
    (Effects|SpawnEmitteratLocation "/Game/FXVarietyPack/Particles/P_ky_explosion.P_ky_explosion" (Transformation|GetActorLocation) "0.000000,90.000000, 0" (Math|Conversions|ToVector(Float) (* 0.1 (Variables|Default|GetCarbineChargeValue))))
    (bind _asork_character (Utilities|Casting|CastToOrk_Character OtherActor))
    (if (and (not (Variables|/Script/WH40K.Ork_Character|GetIsStunned _asork_character)) (>= (Variables|Default|GetCarbineChargeValue) 5e+01))
      (bind _asork_character_2 (Utilities|Casting|CastToOrk_Character OtherActor))
      (Variables|/Script/WH40K.Ork_Character|SetIsStunned _asork_character_2 true))
    (Class|BPINPC|HitbyRecoil(Message) OtherActor (Variables|Default|GetDamage))
    (Actor|DestroyActor)
    (else
      (Effects|SpawnEmitteratLocation "/Game/FXVarietyPack/Particles/P_ky_explosion.P_ky_explosion" "0, 0, 0" "0.000000,90.000000, 0"))))

(event EventBeginPlay
  (bind _carbinechargevalue (Variables|Default|GetCarbineChargeValue))
  (bind _returnvalue (/ _carbinechargevalue 1e+01))
  (Variables|Default|SetDamage (* (Variables|Default|GetDamage) _returnvalue))
  (Transformation|SetActorScale3D (Math|Conversions|ToVector(Float) _returnvalue))
  (Utilities|FlowControl|Delay 1e+01)
  (Actor|DestroyActor))

(event Collision|EventActorBeginOverlap
  (params (OtherActor :type Actor%20Object%20Reference)))

(event EventTick
  (params (DeltaSeconds :type Float%20%28single-precision%29)))

(fn ConstructionScript)