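; Projectile actor that damages enemies through a message and cleans itself up after a ten-second lifetime.
; On capsule overlap it checks the sweep result's hit actor for the Enemy tag, then spawns a character-hit effect, sends HitByRecoilMessage to the overlapped actor and destroys itself.
; Other overlaps only spawn a world-hit effect, leaving the projectile alive.
; Unconnected leftover nodes for killing Enemy_Bp and firing a radial impulse never run.
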(event OnComponentBeginOverlap(Capsule)
  (params (OverlappedComponent :type Primitive%20Component%20Object%20Reference) (OtherActor :type Actor%20Object%20Reference) (OtherComp :type Primitive%20Component%20Object%20Reference) (OtherBodyIndex :type Integer) (bFromSweep :type Boolean) (SweepResult :type Hit%20Result%20Structure%20%28by%20ref%29))
  (if (Actor|ActorHasTag (.HitActor (Collision|BreakHitResult SweepResult)) "Enemy")
    (Effects|SpawnEmitteratLocation "/Game/FireCaste/FX/Particles/Abilities/ScopedShot/FX/P_Wraith_Sniper_HitCharacter.P_Wraith_Sniper_HitCharacter" (Transformation|GetActorLocation) "0.000000,90.000000, 0" "0.100000,0.100000,0.100000")
    (Class|BPINPC|HitbyRecoil(Message) OtherActor)
    (Actor|DestroyActor)
    (else
      (Effects|SpawnEmitteratLocation "/Game/FireCaste/P_Carbine_HitWorld.P_Carbine_HitWorld" (Transformation|GetActorLocation)))))

(event EventBeginPlay
  (Utilities|FlowControl|Delay 1e+01)
  (Actor|DestroyActor))

(event Collision|EventActorBeginOverlap
  (params (OtherActor :type Actor%20Object%20Reference)))

(event EventTick
  (params (DeltaSeconds :type Float%20%28single-precision%29)))

(fn ConstructionScript)