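; MyShieldDrone is a temporary shield drone that turns with the player and destroys "Shoota"-tagged actors entering its shield collision.
; It plays a spawn sound, sets a 45-second lifespan, then after a short delay reveals its mesh and sets its floating movement speed.
; Player overlap activates the shield effect and audio, while Tick smoothly interpolates yaw toward the player's.
; On destruction it calls DelayDrone on the Fire Warrior character and spawns teleport particles and sound.
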(event OnComponentBeginOverlap(ShieldCollision)
  (params (OverlappedComponent :type Primitive%20Component%20Object%20Reference) (OtherActor :type Actor%20Object%20Reference) (OtherComp :type Primitive%20Component%20Object%20Reference) (OtherBodyIndex :type Integer) (bFromSweep :type Boolean) (SweepResult :type Hit%20Result%20Structure%20%28by%20ref%29))
  (Utilities|IsValid OtherActor
    (:Is%20Valid
      (if (Actor|ActorHasTag OtherActor "Player")
        (Components|Activation|SetActive (Variables|Default|GetShieldEffect) true false)
        (Components|Activation|SetActive (Variables|Default|GetShieldAudioComponent) true false)
        (elif (Actor|ActorHasTag OtherActor "Shoota")
          (Actor|DestroyActor OtherActor))))))

(event EventBeginPlay
  (Audio|SpawnSoundatLocation "/Game/Audio/Whoosh_Transition_049_Cue.Whoosh_Transition_049_Cue" (Transformation|GetActorLocation) "0, 0, 0" 0.4 1.0 0.0 0 0)
  (Actor|SetLifeSpan 45.0)
  (Utilities|FlowControl|Delay 1.2)
  (Rendering|SetVisibility (Variables|Default|GetDroneMesh) true false)
  (Variables|/Script/Engine.FloatingPawnMovement|SetMaxSpeed (Variables|Default|GetFloatingMovement) 6e+02))

(event Collision|EventActorBeginOverlap
  (params (OtherActor :type Actor%20Object%20Reference)))

(event EventTick
  (params (DeltaSeconds :type Float%20%28single-precision%29))
  (Transformation|SetActorRotation (Math|Rotator|MakeRotator 0.0 0.0 (.Yaw (Math|Rotator|BreakRotator (Math|Interpolation|RInterpTo (Transformation|GetActorRotation) (Transformation|GetActorRotation (Game|GetPlayerCharacter 0)) (Utilities|Time|GetWorldDeltaSeconds) 0.6))))))

(event EventDestroyed
  (bind _asmy_fire_warrior_character (Utilities|Casting|CastToMyFireWarrior_Character (Game|GetPlayerCharacter 0)))
  (Default|DelayDrone _asmy_fire_warrior_character)
  (Effects|SpawnEmitteratLocation "/Game/FireCaste/FX/Particles/Abilities/TeleportTarget/FX/P_Wraith_Teleport_Orb.P_Wraith_Teleport_Orb" (Transformation|GetWorldLocation (Variables|Default|GetDroneMesh)) "0, 0, 0" "10.000000,10.000000,10.000000")
  (Audio|SpawnSoundatLocation "/Game/Audio/Whoosh_Transition_049_Cue.Whoosh_Transition_049_Cue" (Transformation|GetActorLocation) "0, 0, 0" 0.4 1.0 0.0 0 0))

(fn ConstructionScript)